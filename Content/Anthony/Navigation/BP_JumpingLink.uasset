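; Smart nav link proxy that makes AI agents jump to the other side when they reach it.
; The construction script derives start and end locations by adding the first point link's offsets to the actor location.
; When an agent implementing BPI_AIJump arrives, the nearer endpoint determines travel direction.
; Upward or level crossings send a jump message with destination and duration; downward ones do so only when ForceJump is set.
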(event `self.ReceiveBeginPlay`)

(event `self.ReceiveSmartLinkReached`
  (params (Agent :type "Actor Object Reference") (Destination :type "Vector Structure (by ref)"))
  (bind (_endlocation_x _endlocation_y _endlocation_z) (`KismetMathLibrary.BreakVector` (`self.EndLocation`)))
  (bind (_startlocation_x _startlocation_y _startlocation_z) (`KismetMathLibrary.BreakVector` (`self.StartLocation`)))
  (bind (_endlocation_x_2 _endlocation_y_2 _endlocation_z_2) (`KismetMathLibrary.BreakVector` (`self.EndLocation`)))
  (bind (_startlocation_x_2 _startlocation_y_2 _startlocation_z_2) (`KismetMathLibrary.BreakVector` (`self.StartLocation`)))
  (bind (_returnvalue_x _returnvalue_y _returnvalue_z) (`KismetMathLibrary.BreakVector` (`self.K2_GetActorLocation` (`self.Agent`))))
  (if (`KismetSystemLibrary.DoesImplementInterface` Agent "/Game/Anthony/Characters/Enemy/AI/Interfaces/BPI_AIJump.BPI_AIJump_C")
    (set `self.Agent` Agent)
    (set `self.DestinationLocation` (`KismetMathLibrary.MakeVector` Destination_X Destination_Y Destination_Z))
    (if (`self.CalculateJumpDirection` (`KismetMathLibrary.MakeVector` _returnvalue_x _returnvalue_y _returnvalue_z))
      (if (<= _startlocation_z_2 _endlocation_z)
        (message `/Game/Anthony/Characters/Enemy/AI/Interfaces/BPI_AIJump.JumpToDestination` (`self.Agent`) (`self.DestinationLocation`) (`self.JumpDuration`) :!label _label)
        (else
          (if (`self.ForceJump`) :!label _label_2
            (goto _label))))
      (elif (<= _endlocation_z_2 _startlocation_z)
        (goto _label)
        (else
          (goto _label_2))))))

(fn `CalculateJumpDirection`
  (params (ActorLocation :type "Vector Structure"))
  (returns (JumpDirection :type Boolean))
  (return (< (`KismetMathLibrary.Vector_Distance` ActorLocation (`self.StartLocation`)) (`KismetMathLibrary.Vector_Distance` ActorLocation (`self.EndLocation`)))))

(fn `UserConstructionScript`
  (bind _returnvalue (`self.K2_GetActorLocation`))
  (bind _pointlinks (`self.PointLinks`))
  (bind (_output_left _output_right) (break `NavigationLink` (`|GetArrayItem` _pointlinks)))
  (if (`KismetArrayLibrary.Array_IsNotEmpty` _pointlinks)
    (set `self.StartLocation` (+ _output_left _returnvalue))
    (set `self.EndLocation` (+ _returnvalue _output_right))))