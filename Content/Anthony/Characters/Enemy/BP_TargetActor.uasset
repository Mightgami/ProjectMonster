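; BP_TargetActor is an enemy-folder actor that periodically jumps to random points around where it started.
; On BeginPlay it stores its start location and starts a looping timer at the ChangeTimer interval.
; Each tick of that timer applies random X and Z offsets within plus or minus Radius, leaving the Y input unset.
; The construction script draws a debug sphere of that Radius.
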(event `self.ReceiveBeginPlay`
  (set `self.StartLocation` (`self.K2_GetActorLocation`))
  (`KismetSystemLibrary.K2_SetTimerDelegate` (delegate `ChangeLocation`) (`self.ChangeTimer`) true))

(event `ChangeLocation`
  (bind _radius (`self.Radius`))
  (bind _returnvalue (* _radius -1.0))
  (bind (_returnvalue_x _returnvalue_y _returnvalue_z) (`KismetMathLibrary.BreakVector` (+ (`self.StartLocation`) (`KismetMathLibrary.MakeVector` (`KismetMathLibrary.RandomFloatInRange` _returnvalue _radius) 0.0 (`KismetMathLibrary.RandomFloatInRange` _returnvalue _radius)))))
  (`self.K2_SetActorLocation` (`KismetMathLibrary.MakeVector` _returnvalue_x 0.0 _returnvalue_z)))

(fn `UserConstructionScript`
  (`KismetSystemLibrary.DrawDebugSphere` (`self.K2_GetActorLocation`) (`self.Radius`)))