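; Base NPC AI controller that runs a behavior tree after a short delay on BeginPlay.
; Perception updates feed sight of the player into the Blackboard: TargetActor receives the player whether sensed or lost, as both select inputs match.
; On sight loss, LastKnownLocation becomes a random reachable point near the stimulus.
; CalculateJumpVelocity solves a ballistic launch velocity from the pawn to Destination for a given duration under fixed gravity.
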(event `self.ReceiveBeginPlay`
  (`KismetSystemLibrary.Delay` 1.0)
  (`self.RunBehaviorTree` (`self.BehaviorTree`)))

(event `self.AIPerception.OnTargetPerceptionUpdated`
  (params (Actor :type "Actor Object Reference") (Stimulus :type "AIStimulus Structure"))
  (`/Engine/EditorBlueprintResources/StandardMacros.IsValid` (`self.Blackboard`)
    (:`Is Valid`
      (`self.HandleSightSense` Actor Stimulus))))

(fn `CalculateJumpVelocity`
  (params (Destination :type "Vector Structure") (JumpDuration :type "Float (double-precision)"))
  (returns (Velocity :type "Vector Structure"))
  (bind _jumpduration (`local.JumpDuration`))
  (bind (_returnvalue_x _returnvalue_y _returnvalue_z) (`KismetMathLibrary.BreakVector` (`self.K2_GetActorLocation` (`self.K2_GetPawn`))))
  (return (`KismetMathLibrary.MakeVector` (`KismetMathLibrary.SafeDivide` (- Destination_X _returnvalue_x) _jumpduration) (`KismetMathLibrary.SafeDivide` (- Destination_Y _returnvalue_y) _jumpduration) (`KismetMathLibrary.SafeDivide` (- Destination_Z (+ _returnvalue_z (* (`KismetMathLibrary.Square` (`local.JumpDuration`)) 0.5 -982.0))) _jumpduration))))

(fn `HandleSightSense`
  (params (Actor :type "Actor Object Reference") (Stimulus :type "AIStimulus Structure"))
  (bind _returnvalue (`GameplayStatics.GetPlayerCharacter` 0))
  (bind (_stimulus_age _stimulus_expirationage _stimulus_strength _stimulus_stimuluslocation _stimulus_receiverlocation _stimulus_tag _stimulus_bsuccessfullysensed) (break `AIStimulus` (`local.Stimulus`)))
  (bind _returnvalue_2 (`AIPerceptionSystem.GetSenseClassForStimulus` Stimulus))
  (if (== _returnvalue_2 "/Script/AIModule.AISense_Sight")
    (if (== (`local.Actor`) (`GameplayStatics.GetPlayerCharacter` 0))
      (`BlackboardComponent.SetValueAsObject` (`self.Blackboard`) "TargetActor" (`KismetMathLibrary.SelectObject` _returnvalue _returnvalue _stimulus_bsuccessfullysensed))
      (if (not _stimulus_bsuccessfullysensed)
        (`BlackboardComponent.SetValueAsVector` (`self.Blackboard`) "LastKnownLocation" (`NavigationSystemV1.K2_GetRandomReachablePointInRadius` _stimulus_stimuluslocation 100.0 null null)))
      (else
        (return)))
    (else
      (return))))

(fn `UserConstructionScript`)