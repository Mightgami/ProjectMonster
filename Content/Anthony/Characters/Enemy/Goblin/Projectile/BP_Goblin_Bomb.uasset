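; Goblin bomb projectile that explodes when a timer runs out or, optionally, on first overlap with the player pawn.
; On BeginPlay it gets a launch impulse on its collision sphere and starts the fuse timer.
; Exploding stops physics, collision and movement, resets rotation and jumps the animation state; damage is only a debug print placeholder.
; The construction script keeps X and Z and zeroes Y, snapping it to a 2D plane.
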(event `self.ReceiveBeginPlay`
  ; BeginPlay
  (`PrimitiveComponent.AddImpulse` (`self.SphereCollision`) (`self.BeginImpulse`) "None" true)
  (bind _returnvalue (`KismetSystemLibrary.K2_SetTimerDelegate` (delegate `Explode`) (`self.ExplosionTime`)))
  (set `self.ExplosionTimer` _returnvalue)
  (set `PrimitiveComponent.bGenerateOverlapEvents` true (`self.SphereCollision`)))

(event `Explode`
  (bind _spherecollision (`self.SphereCollision`))
  (`KismetSystemLibrary.K2_ClearAndInvalidateTimerHandle` (`self.ExplosionTimer`))
  (`PrimitiveComponent.SetSimulatePhysics` _spherecollision false)
  (`PrimitiveComponent.SetCollisionEnabled` _spherecollision "NoCollision")
  (`ActorComponent.Deactivate` (`self.ProjectileMovement`))
  (`self.K2_SetActorRotation` (struct))
  (`PaperZDAnimInstance.JumpToNode` (`PaperZDAnimationComponent.AnimInstance` (`self.AnimationComponent`)) "TimeFinished" "None")
  (`KismetSystemLibrary.PrintString` "BP_Goblin_Bomb_Add Damage"))

(event `self.SphereCollision.OnComponentBeginOverlap`
  (params (OverlappedComponent :type "PrimitiveComponent Object Reference") (OtherActor :type "Actor Object Reference") (OtherComp :type "PrimitiveComponent Object Reference") (OtherBodyIndex :type Integer) (bFromSweep :type Boolean) (SweepResult :type "HitResult Structure (by ref)"))
  (if (and (`self.ShouldExplodeOnContact`) (== OtherActor (`GameplayStatics.GetPlayerPawn` 0)))
    (`/Engine/EditorBlueprintResources/StandardMacros.DoOnce` false
      (:`Completed`
        (`self.Explode`)))))

(fn `UserConstructionScript`
  (bind (_returnvalue_x _returnvalue_y _returnvalue_z) (`KismetMathLibrary.BreakVector` (`self.K2_GetActorLocation`)))
  (`self.K2_SetActorLocation` (`KismetMathLibrary.MakeVector` _returnvalue_x 0.0 _returnvalue_z)))