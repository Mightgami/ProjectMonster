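; Goblin AI controller that decides whether its navigation may use jumps.
; On BeginPlay it checks whether the controlled pawn implements the BPI_AIJump interface.
; It then sets the default navigation filter to the jump-include or jump-exclude class accordingly, printing which one applies for debugging.
; Tick is disabled and the construction script only calls its parent.
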(event `self.ReceiveBeginPlay`
  (`parent.ReceiveBeginPlay`)
  (if (`KismetSystemLibrary.DoesImplementInterface` (`self.K2_GetPawn`) "/Game/Anthony/Characters/Enemy/AI/Interfaces/BPI_AIJump.BPI_AIJump_C")
    (set `self.DefaultNavigationFilterClass` "/Game/Anthony/Navigation/NavMeshFilter/NFQ_JumpInclude.NFQ_JumpInclude_C")
    (`KismetSystemLibrary.PrintString` "HasJump")
    (else
      (set `self.DefaultNavigationFilterClass` "/Game/Anthony/Navigation/NavMeshFilter/NFQ_JumpExclude.NFQ_JumpExclude_C")
      (`KismetSystemLibrary.PrintString` "NoJump"))))

(fn `UserConstructionScript`
  (`parent.UserConstructionScript`))