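; BP_Skeleton is a skeleton enemy character that can jump to a given destination in a set time.
; Its JumptoDestination event feeds the destination and duration into CalculateJumpVelocity, then launches the character, overriding its current velocity on all axes.
; The helper solves a ballistic arc: constant horizontal speed, with vertical speed compensating for a hard-coded gravity of -982.
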(event `self.JumpToDestination`
  (params (`Destination Location` :type "Vector Structure") (JumpDuration :type "Float (double-precision)"))
  (bind _velocity (`self.CalculateJumpVelocity` `Destination Location` JumpDuration))
  (`self.LaunchCharacter` _velocity true true))

(fn `CalculateJumpVelocity`
  (params (Destination :type "Vector Structure") (JumpDuration :type "Float (double-precision)"))
  (returns (Velocity :type "Vector Structure"))
  (bind (_returnvalue_x _returnvalue_y _returnvalue_z) (`KismetMathLibrary.BreakVector` (`self.K2_GetActorLocation`)))
  (bind _jumpduration (`local.JumpDuration`))
  (return (`KismetMathLibrary.MakeVector` (`KismetMathLibrary.SafeDivide` (- Destination_X _returnvalue_x) _jumpduration) (`KismetMathLibrary.SafeDivide` (- Destination_Y _returnvalue_y) _jumpduration) (`KismetMathLibrary.SafeDivide` (- Destination_Z (+ _returnvalue_z (* (`KismetMathLibrary.Square` (`local.JumpDuration`)) 0.5 -982.0))) _jumpduration))))

(fn `UserConstructionScript`
  (`parent.UserConstructionScript`))