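; Character Blueprint that drives airborne animation and switches between Warrior, Ranger and Mage animation sets.
; Jumping and walking off a ledge share one path that clears IsLanded and makes the anim instance jump directly to its "Airbone" node.
; Landing only sets IsLanded back to true.
; Number keys swap the AnimationComponent's Anim Instance class at runtime to change between the three sets.
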(event `self.OnJumped`
  (set `self.IsLanded` false :!label _label)
  (`PaperZDAnimInstance.JumpToNode` (`PaperZDAnimationComponent.AnimInstance` (`self.AnimationComponent`)) "Airbone" "None"))

(event `self.OnWalkingOffLedge`
  (params (PreviousFloorImpactNormal :type "Vector Structure (by ref)") (PreviousFloorContactNormal :type "Vector Structure (by ref)") (PreviousLocation :type "Vector Structure (by ref)") (TimeDelta :type "Float (single-precision)"))
  (goto _label))

(event `self.OnLanded`
  (params (Hit :type "HitResult Structure (by ref)"))
  (set `self.IsLanded` true))

(event `Key|One`
  (params (Key :type "Key Structure"))
  (:`Pressed`
    (`PaperZDAnimationComponent.SetAnimInstanceClass` (`self.AnimationComponent`) "/Game/Blueprints/Characters/Warrior/Animations/ABP_Warrior.ABP_Warrior_C")))

(event `Key|Two`
  (params (Key :type "Key Structure"))
  (:`Pressed`
    (`PaperZDAnimationComponent.SetAnimInstanceClass` (`self.AnimationComponent`) "/Game/Blueprints/Characters/Ranger/ABP_Ranger.ABP_Ranger_C")))

(event `Key|Three`
  (params (Key :type "Key Structure"))
  (:`Pressed`
    (`PaperZDAnimationComponent.SetAnimInstanceClass` (`self.AnimationComponent`) "/Game/Blueprints/Characters/Mage/ABP_Mage.ABP_Mage_C")))

(fn `UserConstructionScript`)